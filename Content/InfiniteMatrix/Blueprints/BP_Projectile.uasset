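; BP_Projectile is the player's projectile, which flies along world X and scores points by destroying enemies.
; Each tick it sweeps forward at the player's forward speed plus a bonus speed.
; When its hitbox overlaps a component tagged ProjectileHittable, a tunnel breaks only the projectile, while an enemy is broken too and increments the player's score.
; Breaking spawns a burst particle system at its center and destroys the actor.
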(event `self.ReceiveTick`
  (params (DeltaSeconds :type "Float (single-precision)"))
  (`self.K2_AddActorWorldOffset` (`KismetMathLibrary.MakeVector` (* DeltaSeconds (+ (`self.BonusSpeed`) (`/Game/InfiniteMatrix/Blueprints/BP_Player.ForwardSpeed` (`self.Player`))))) true))

(event `self.Hitbox.OnComponentBeginOverlap`
  (params (OverlappedComponent :type "PrimitiveComponent Object Reference") (OtherActor :type "Actor Object Reference") (OtherComp :type "PrimitiveComponent Object Reference") (OtherBodyIndex :type Integer) (bFromSweep :type Boolean) (SweepResult :type "HitResult Structure (by ref)"))
  (`/Engine/EditorBlueprintResources/StandardMacros.IsValid` (`self.Player`)
    (:`Is Valid`
      (if (`ActorComponent.ComponentHasTag` OtherComp "ProjectileHittable")
        (cast `/Game/InfiniteMatrix/Blueprints/BP_Tunnel` OtherActor
          (:`then`
            (`self.Break`))
          (:`CastFailed`
            (bind _asbp_enemy (cast `/Game/InfiniteMatrix/Blueprints/BP_Enemy` OtherActor))
            (`/Game/InfiniteMatrix/Blueprints/BP_Enemy.Break` _asbp_enemy)
            (`/Game/InfiniteMatrix/Blueprints/BP_Player.IncrementScore` (`self.Player`))
            (`self.Break`)))))))

(fn `Break`
  (`NiagaraFunctionLibrary.SpawnSystemAtLocation` "/Game/InfiniteMatrix/Particles/ProjectileBurst.ProjectileBurst" (`SceneComponent.K2_GetComponentLocation` (`self.Center`)))
  (`self.K2_DestroyActor`))

(fn `UserConstructionScript`)