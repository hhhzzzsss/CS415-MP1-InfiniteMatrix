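; Endless-tunnel segment with a randomized, spinning holed wall that damages BP_Player on contact.
; RandomizeWall picks mesh, angle and spin, while SpawnEntities scatters an occasional health pack and enemies using disc-style offsets, rejecting overlapping enemies.
; Player entry into TriggerZone asks TunnelSpawner for another segment, then destroys this one and its entities.
; TriggerZone end overlap awards score if the wall was not hit.
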(event `self.ReceiveTick`
  (params (DeltaSeconds :type "Float (single-precision)"))
  (`SceneComponent.K2_AddLocalRotation` (`self.WallMesh`) (`KismetMathLibrary.MakeRotator` (* DeltaSeconds (`self.RotateSpeed`))) false false))

(event `self.TriggerZone.OnComponentBeginOverlap`
  (params (OverlappedComponent :type "PrimitiveComponent Object Reference") (OtherActor :type "Actor Object Reference") (OtherComp :type "PrimitiveComponent Object Reference") (OtherBodyIndex :type Integer) (bFromSweep :type Boolean) (SweepResult :type "HitResult Structure (by ref)"))
  (cast `/Game/InfiniteMatrix/Blueprints/BP_Player` OtherActor)
  (`/Game/InfiniteMatrix/Blueprints/BP_TunnelSpawner.SpawnTunnelAtSpawnPoint` (`self.TunnelSpawner`))
  (`self.DestroyEntities`)
  (`self.K2_DestroyActor`))

(event `self.WallMesh.OnComponentBeginOverlap`
  (params (OverlappedComponent :type "PrimitiveComponent Object Reference") (OtherActor :type "Actor Object Reference") (OtherComp :type "PrimitiveComponent Object Reference") (OtherBodyIndex :type Integer) (bFromSweep :type Boolean) (SweepResult :type "HitResult Structure (by ref)"))
  (bind _asbp_player (cast `/Game/InfiniteMatrix/Blueprints/BP_Player` OtherActor))
  (`/Game/InfiniteMatrix/Blueprints/BP_Player.Take Damage` _asbp_player)
  (set `self.WasHit` true))

(event `self.TriggerZone.OnComponentEndOverlap`
  (params (OverlappedComponent :type "PrimitiveComponent Object Reference") (OtherActor :type "Actor Object Reference") (OtherComp :type "PrimitiveComponent Object Reference") (OtherBodyIndex :type Integer))
  (bind _asbp_player (cast `/Game/InfiniteMatrix/Blueprints/BP_Player` OtherActor))
  (if (not (`self.WasHit`))
    (`/Game/InfiniteMatrix/Blueprints/BP_Player.IncrementScore` _asbp_player)))

(fn `DestroyEntities`
  (bind _healthpack (`self.HealthPack`))
  (`|ExecutionSequence`
    (:`then_0`
      (`/Engine/EditorBlueprintResources/StandardMacros.IsValid` _healthpack
        (:`Is Valid`
          (`self.K2_DestroyActor` _healthpack))))
    (:`then_1`
      (for _array_element (`self.Enemies`)
        (`/Engine/EditorBlueprintResources/StandardMacros.IsValid` _array_element
          (:`Is Valid`
            (`self.K2_DestroyActor` _array_element)))))))

(fn `RandomizeWall`
  (`StaticMeshComponent.SetStaticMesh` (`self.WallMesh`) (select `int` (`KismetMathLibrary.RandomIntegerInRange` 0 3) :`0` "/Game/InfiniteMatrix/Meshes/SM_Hole_01.SM_Hole_01" :`1` "/Game/InfiniteMatrix/Meshes/SM_Hole_02.SM_Hole_02" :`2` "/Game/InfiniteMatrix/Meshes/SM_Hole_03.SM_Hole_03" :`3` "/Game/InfiniteMatrix/Meshes/SM_Hole_04.SM_Hole_04" :!type "StaticMesh Object Reference"))
  (`SceneComponent.K2_AddLocalRotation` (`self.WallMesh`) (`KismetMathLibrary.MakeRotator` (`KismetMathLibrary.RandomFloatInRange` 0.0 360.0)) false false)
  (set `self.RotateSpeed` (`KismetMathLibrary.RandomFloatInRange` -50.0 50.0)))

(fn `SpawnEnemy`
  (bind _returnvalue (* (`KismetMathLibrary.MultiplyByPi` (`KismetMathLibrary.RandomFloat`)) 2.0))
  (bind _returnvalue_2 (* (`KismetMathLibrary.Sqrt` (`KismetMathLibrary.RandomFloat`)) 360.0))
  (bind _returnvalue_3 (`|SpawnActorFromClass` "/Game/InfiniteMatrix/Blueprints/BP_Enemy.BP_Enemy_C" (`KismetMathLibrary.MakeTransform` (+ (`SceneComponent.K2_GetComponentLocation` (`self.Center`)) (`KismetMathLibrary.MakeVector` (`KismetMathLibrary.RandomFloatInRange` -1000.0 1000.0) (* (`KismetMathLibrary.Sin` _returnvalue) _returnvalue_2) (* (`KismetMathLibrary.Cos` _returnvalue) _returnvalue_2)))) "Undefined" "MultiplyWithRoot" null null))
  (if (and (`KismetArrayLibrary.Array_IsEmpty` (`self.GetOverlappingActors` _returnvalue_3 "/Game/InfiniteMatrix/Blueprints/BP_HealthPack.BP_HealthPack_C")) (`KismetArrayLibrary.Array_IsEmpty` (`self.GetOverlappingActors` _returnvalue_3 "/Game/InfiniteMatrix/Blueprints/BP_Enemy.BP_Enemy_C")))
    (`KismetArrayLibrary.Array_Add` (`self.Enemies`) _returnvalue_3)
    (else
      (`self.K2_DestroyActor` _returnvalue_3)
      (`KismetSystemLibrary.PrintString` "Destroyed Overlapping Enemy"))))

(fn `SpawnEntities`
  (`|ExecutionSequence`
    (:`then_0`
      (if (== (`KismetMathLibrary.RandomIntegerInRange` 0 3) 0)
        (`self.SpawnHealthPack`)))
    (:`then_1`
      (for _ (range (+ (`KismetMathLibrary.RandomIntegerInRange` 0 2) 1))
        (`self.SpawnEnemy`)))))

(fn `SpawnHealthPack`
  (bind _returnvalue (* (`KismetMathLibrary.MultiplyByPi` (`KismetMathLibrary.RandomFloat`)) 2.0))
  (bind _returnvalue_2 (* (`KismetMathLibrary.Sqrt` (`KismetMathLibrary.RandomFloat`)) 400.0))
  (bind _returnvalue_3 (`|SpawnActorFromClass` "/Game/InfiniteMatrix/Blueprints/BP_HealthPack.BP_HealthPack_C" (`KismetMathLibrary.MakeTransform` (+ (`SceneComponent.K2_GetComponentLocation` (`self.Center`)) (`KismetMathLibrary.MakeVector` (`KismetMathLibrary.RandomFloatInRange` -300.0 600.0) (* (`KismetMathLibrary.Sin` _returnvalue) _returnvalue_2) (* (`KismetMathLibrary.Cos` _returnvalue) _returnvalue_2)))) "Undefined" "MultiplyWithRoot" null null))
  (set `self.HealthPack` _returnvalue_3))

(fn `UserConstructionScript`)