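; Post-process actor that drives a screen vignette effect which fades out over time.
; The construction script creates a dynamic instance of M_Vignette, adds it as a blendable to the PostProcess component and stores it.
; Helper functions get and set the vignette strength and set its color on that instance.
; Tick lowers the strength at a constant rate down to zero, so any raised value acts as a brief pulse.
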(event `self.ReceiveTick`
  (params (DeltaSeconds :type "Float (single-precision)"))
  (bind _vignettestrength (`self.GetVignetteStrength`))
  (`self.SetVignetteStrength` (`KismetMathLibrary.FMax` (- _vignettestrength (* DeltaSeconds 2.0)))))

(fn `GetVignetteStrength`
  (returns (VignetteStrength :type "Float (double-precision)"))
  (bind _returnvalue (`MaterialInstanceDynamic.K2_GetScalarParameterValue` (`self.Vignette`) "Vignette Strength"))
  (return _returnvalue))

(fn `SetVignetteColor`
  (params (VignetteColor :type "LinearColor Structure"))
  (`MaterialInstanceDynamic.SetVectorParameterValue` (`self.Vignette`) "Vignette Color" VignetteColor))

(fn `SetVignetteStrength`
  (params (VignetteStrength :type "Float (double-precision)"))
  (`MaterialInstanceDynamic.SetScalarParameterValue` (`self.Vignette`) "Vignette Strength" VignetteStrength))

(fn `UserConstructionScript`
  (bind _returnvalue (`KismetMaterialLibrary.CreateDynamicMaterialInstance` "/Game/InfiniteMatrix/Materials/M_Vignette.M_Vignette"))
  (`PostProcessComponent.AddOrUpdateBlendable` (`self.PostProcess`) _returnvalue 1.0)
  (set `self.Vignette` _returnvalue))